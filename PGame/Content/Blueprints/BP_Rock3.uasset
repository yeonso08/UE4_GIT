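; BP_Rock3 is a rock actor whose Cube component moves up and down continuously.
; Tick accumulates delta seconds into a Time variable and feeds it through a scaled sine to offset the Cube's world Z, keeping X and Y unchanged.
; The offset is added to the current position each frame rather than a stored origin, so the travel range depends on frame rate.
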(event `self.ReceiveTick`
  (params (DeltaSeconds :type "Float (single-precision)"))
  (bind _output_get (set `self.Time` (+ DeltaSeconds (`self.Time`))))
  (bind _output_get_2 (set `self.Location` (`KismetMathLibrary.MakeVector` (.x (`SceneComponent.K2_GetComponentLocation` (`self.Cube`))) (.y (`SceneComponent.K2_GetComponentLocation` (`self.Cube`))) (+ (* (`KismetMathLibrary.Sin` _output_get) -30.0) (.z (`SceneComponent.K2_GetComponentLocation` (`self.Cube`)))))))
  (`SceneComponent.K2_SetWorldLocation` (`self.Cube`) _output_get_2 false false))

(fn `UserConstructionScript`)